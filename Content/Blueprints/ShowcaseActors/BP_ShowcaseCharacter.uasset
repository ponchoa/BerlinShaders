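; Showcase player character that highlights interactable actors and sets up a see-through-walls view.
; Each tick, a camera line trace toggles custom depth on the looked-at actor tagged "Interact".
; A scene capture, limited to itself and "WallHack"-tagged actors, renders to a viewport-sized target fed into a camera post-process material.
; Functions also toggle that capture and call Interact on stored interactables.
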(event EventTick
  (params (DeltaSeconds :type Float%20%28single-precision%29))
  (Rendering|HighlightInteract))

(event EventBeginPlay
  (Utilities|FlowControl|Delay 0.2)
  (Rendering|CustomViewSetup)
  (Rendering|SetRenderView "WallHack"))

(fn ConstructionScript)

(fn SetCustomDepthPass
  (params (Enable :type Boolean) (Actor%20To%20Render :type Actor%20Object%20Reference%20%28by%20ref%29))
  (bind _returnvalue (Actor|GetComponentsByClass Actor%20To%20Render "/Script/Engine.PrimitiveComponent"))
  (if (<= 0 (Utilities|Array|Length _returnvalue))
    (for _array_element _returnvalue
      (Rendering|SetRenderCustomDepth _array_element Enable))
    (return true)
    (else
      (return false))))

(fn HighlightInteract
  (bind _playercamera (Variables|Default|GetPlayerCamera))
  (bind _returnvalue (Transformation|GetWorldLocation _playercamera))
  (bind (_outhit _returnvalue_2) (Collision|LineTraceByChannel _returnvalue (+ _returnvalue (* (Math|Vector|GetForwardVector _playercamera) (Variables|Gameplay|GetInteract%20Distance))) "TraceTypeQuery1" true 0 "None"))
  (if _returnvalue_2
    (Utilities|IsValid (.HitActor (Collision|BreakHitResult _outhit))
      (:Is%20Valid
        (if (Utilities|IsValid (Variables|Rendering|GetLooked%20At%20Actor))
          (if (!= (Variables|Rendering|GetLooked%20At%20Actor) (.HitActor (Collision|BreakHitResult _outhit)))
            (Rendering|SetCustomDepthPass false (Variables|Rendering|GetLooked%20At%20Actor))
            (if (Actor|ActorHasTag (.HitActor (Collision|BreakHitResult _outhit)) "Interact") :!label _label
              (bind _success (Rendering|SetCustomDepthPass true (.HitActor (Collision|BreakHitResult _outhit))))
              (if _success
                (Variables|Rendering|SetLooked%20At%20Actor (.HitActor (Collision|BreakHitResult _outhit)))
                (else
                  (Variables|Rendering|SetLooked%20At%20Actor 0 :!label _label_2)))
              (else
                (goto _label_2))))
          (else
            (goto _label))))
      (:Is%20Not%20Valid
        (if (Utilities|IsValid (Variables|Rendering|GetLooked%20At%20Actor)) :!label _label_3
          (Rendering|SetCustomDepthPass false (Variables|Rendering|GetLooked%20At%20Actor))
          (goto _label_2))))
    (else
      (goto _label_3))))

(fn CustomViewSetup
  (bind _returnvalue (Viewport|GetViewportSize))
  (bind _returnvalue_2 (Rendering|CreateRenderTarget2D (Math|Float|Truncate (.x _returnvalue)) (Math|Float|Truncate (.y _returnvalue)) "RTF_RGBA16f"))
  (bind _output_get (Variables|/Script/Engine.SceneCaptureComponent2D|SetTextureTarget (Variables|Default|GetCustomRenderCapture) _returnvalue_2))
  (bind _returnvalue_3 (Rendering|Material|CreateDynamicMaterialInstance "/Game/Materials/PostProcess/PPM_RenderThroughWall.PPM_RenderThroughWall" "None" "None" :!class /Script/Engine.KismetMaterialLibrary))
  (Rendering|Material|SetTextureParameterValue _returnvalue_3 "Player Render Target" _output_get)
  (Rendering|AddorUpdateBlendable (Variables|Default|GetPlayerCamera) _returnvalue_3 1.0 :!class /Script/Engine.CameraComponent))

(fn SetRenderView
  (params (Tag :type Name :default "None"))
  (bind _outactors (Actor|GetAllActorswithTag Tag))
  (bind _output_get (Variables|/Script/Engine.SceneCaptureComponent|SetShowOnlyActors (Variables|Default|GetCustomRenderCapture) _outactors))
  (Utilities|Array|Add _output_get self))

(fn EnableCustomRender
  (params (Enable :type Boolean))
  (bind _customrendercapture (Variables|Default|GetCustomRenderCapture))
  (Rendering|ClearRenderTarget2D (Variables|/Script/Engine.SceneCaptureComponent2D|GetTextureTarget _customrendercapture))
  (bind _output_get (Variables|/Script/Engine.SceneCaptureComponent|SetbCaptureEveryFrame _customrendercapture Enable))
  (bind _output_get_2 (Variables|/Script/Engine.SceneCaptureComponent|SetbCaptureOnMovement _customrendercapture _output_get))
  (return _output_get_2))

(fn Use
  (if (<= 0 (Utilities|Array|Length (Variables|Gameplay|GetInteractables)))
    (for _array_element (Variables|Gameplay|GetInteractables)
      (Default|Interact _array_element))))