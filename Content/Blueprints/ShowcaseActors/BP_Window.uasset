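; Showcase actor that cycles through three window components when the player character interacts with it.
; The trigger area adds and removes it from BP_ShowcaseCharacter's Interactables list.
; Interact advances the cycle, with a timeline sliding the current and next windows along local X; Switch also supports going backward.
; Custom render on the character is enabled only while it is at the trigger with Window3 showing, and cleared on interact or exit.
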(event OnComponentBeginOverlap(TriggerArea)
  (params (OverlappedComponent :type Primitive%20Component%20Object%20Reference) (OtherActor :type Actor%20Object%20Reference) (OtherComp :type Primitive%20Component%20Object%20Reference) (OtherBodyIndex :type Integer) (bFromSweep :type Boolean) (SweepResult :type Hit%20Result%20Structure%20%28by%20ref%29))
  (bind _asbp_showcase_character (Utilities|Casting|CastToBP_ShowcaseCharacter OtherActor))
  (bind _output_get (Variables|Default|SetCharacter _asbp_showcase_character))
  (Utilities|Array|Add (Variables|/Game/Blueprints/ShowcaseActors/BP_ShowcaseCharacter.BP_ShowcaseCharacter_C|GetInteractables _output_get) self)
  (if (== (Variables|Basic|GetCurrentWindow) (Variables|Default|GetWindow3))
    (Default|EnableCustomRender _output_get true)))

(event OnComponentEndOverlap(TriggerArea)
  (params (OverlappedComponent :type Primitive%20Component%20Object%20Reference) (OtherActor :type Actor%20Object%20Reference) (OtherComp :type Primitive%20Component%20Object%20Reference) (OtherBodyIndex :type Integer))
  (bind _asbp_showcase_character (Utilities|Casting|CastToBP_ShowcaseCharacter OtherActor))
  (Utilities|Array|RemoveItem (Variables|/Game/Blueprints/ShowcaseActors/BP_ShowcaseCharacter.BP_ShowcaseCharacter_C|GetInteractables _asbp_showcase_character) self)
  (Default|EnableCustomRender _asbp_showcase_character false))

(event Custom|Switch
  (params (Backward :type Boolean))
  (bind _returnvalue (Math|Float|SelectFloat -8e+02 8e+02 Backward))
  (bind _window (CallFunction|GetNextWindow Backward))
  (bind _alpha (Timeline|Move PlayFromStart)
    (:Update
      (Transformation|SetRelativeLocation _window (Math|Vector|MakeVector (* (+ _alpha 1.0) _returnvalue) 0.0 0.0) false false)
      (Transformation|SetRelativeLocation (Variables|Basic|GetCurrentWindow) (Math|Vector|MakeVector (* _alpha _returnvalue) 0.0 0.0) false false))
    (:Finished
      (bind _output_get (Variables|Basic|SetCurrentWindow _window))
      (if (== _output_get (Variables|Default|GetWindow3))
        (Default|EnableCustomRender (Variables|Default|GetCharacter) true)))))

(event EventBeginPlay
  (Variables|Basic|SetCurrentWindow (Variables|Default|GetWindow1)))

(event EventInteract
  (CallFunction|Switch false)
  (Default|EnableCustomRender (Variables|Default|GetCharacter) false))

(fn ConstructionScript)

(fn GetNextWindow
  (params (Previous :type Boolean))
  (bind _currentwindow (Variables|Basic|GetCurrentWindow))
  (bind _window3 (Variables|Default|GetWindow3))
  (if (== _currentwindow (Variables|Default|GetWindow1))
    (if Previous
      (return (Variables|Default|GetWindow3))
      (else
        (return (Variables|Default|GetWindow2))))
    (elif (== _currentwindow (Variables|Default|GetWindow2))
      (if Previous
        (return (Variables|Default|GetWindow1))
        (else
          (return (Variables|Default|GetWindow3))))
      (elif (== _window3 _window3)
        (if Previous
          (return (Variables|Default|GetWindow2))
          (else
            (return (Variables|Default|GetWindow1))))))))