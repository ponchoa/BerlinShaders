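; Runs Conway's Game of Life on render targets and shows it through the BP_NadaPawn HUD.
; While running (Space toggles), each tick steps BufferTarget via a GPU compute material or CPU cell map (T switches).
; The CPU path stores only non-zero cells, packing alive bit and neighbor count per byte, updating neighbors and pixels only on state changes.
; A render material draws BufferTarget into DisplayTarget every tick.
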(event EventTick
  (params (DeltaSeconds :type Float%20%28single-precision%29))
  (Utilities|FlowControl|Sequence
    (:then_0
      (if (Variables|Buffers|GetCanEvaluate)
        (if (Variables|Options|GetUse%20GPU)
          (bind (_canvas _size _context) (Rendering|BeginDrawCanvastoRenderTarget (Variables|Buffers|GetBuffer%20Target)))
          (Canvas|DrawMaterial :self _canvas :RenderMaterial (Variables|Materials|GetCompute%20Material) :ScreenSize _size :CoordinateSize "(X=1.000000,Y=1.000000)" :PivotPoint "(X=0.500000,Y=0.500000)")
          (Rendering|EndDrawCanvastoRenderTarget _context)
          (else
            (Processing|ComputeCellBuffer)))))
    (:then_1
      (Rendering|DrawCurrentState))))

(event EventBeginPlay
  (Utilities|FlowControl|Delay 0.1)
  (Init|InitBufferSize)
  (Init|SetupRenderTarget)
  (bind _asbp_nada_pawn (Utilities|Casting|CastToBP_NadaPawn (Game|Player|GetPlayerPawn 0)))
  (Default|SetDisplayTarget (Variables|/Game/Conway/Gamemode/BP_NadaPawn.BP_NadaPawn_C|GetHUD _asbp_nada_pawn) (Variables|Buffers|GetDisplay%20Target)))

(event Input|KeyboardEvents|SpaceBar
  (params (Key :type Key%20Structure :default "None"))
  (:Released
    (Variables|Buffers|SetCanEvaluate (not (Variables|Buffers|GetCanEvaluate)))))

(event Input|KeyboardEvents|T
  (params (Key :type Key%20Structure :default "None"))
  (:Released
    (Variables|Options|SetUse%20GPU (not (Variables|Options|GetUse%20GPU)))))

(fn ConstructionScript)

(fn AreCoordsValid
  (params (Coords :type Int%20Point%20Structure))
  (bind _canvas_size (Variables|Buffers|GetCanvas%20Size))
  (return (and (Math|Integer|InRange(Integer) (.x Coords) 0 (.x _canvas_size) true false) (Math|Integer|InRange(Integer) (.y Coords) 0 (.y _canvas_size) true false))))

(fn BytetoCell
  (params (Value :type Byte))
  (return (Utilities|Struct|MakeS_Cell (Math|Conversions|ToInteger(Byte) (/ Value 2)) (== 1 (Class|KismetMathLibrary|PercentByteByte Value 2)))))

(fn CelltoByte
  (params (Cell :type S%20Cell%20Structure))
  (return (+ (* (Math|Conversions|ToByte(Integer) (Math|Integer|Clamp(Integer) (.n-count Cell) 0 8)) 2) (Math|Integer|SelectInt 1 0 (.alive Cell)))))

(fn GetCell
  (params (Coords :type Int%20Point%20Structure))
  (return (Conversions|BytetoCell (.Value (Utilities|Map|Find (Variables|Buffers|GetCellsBuffer) Coords)))))

(fn SetCell
  (params (Coords :type Int%20Point%20Structure) (Cell :type S%20Cell%20Structure))
  (bind _value (Conversions|CelltoByte Cell))
  (Utilities|Map|Add (Variables|Buffers|GetCellsBuffer) Coords _value)
  (Canvas|DrawTexture :self (Variables|Materials|GetCanvas) :ScreenPosition (Math|Conversions|ToVector2D(IntPoint) Coords) :ScreenSize "(X=1.000000,Y=1.000000)" :CoordinateSize "(X=1.000000,Y=1.000000)" :RenderColor (Math|Color|MakeColor (Math|Conversions|ToFloat(Integer) (Math|Conversions|ToInteger(Byte) _value)) 0.0 0.0) :BlendMode "BLEND_Opaque" :PivotPoint "(X=0.000000,Y=0.000000)")
  (if (> _value 0)
    _
    (else
      (Utilities|Map|Remove (Variables|Buffers|GetCellsBuffer) Coords)))
  (return))

(fn GetCellState
  (params (Coords :type Int%20Point%20Structure))
  (return (.alive (Processing|GetCell Coords))))

(fn SetCellState
  (params (Alive :type Boolean) (Coords :type Int%20Point%20Structure) (Is%20Canvas%20Ready :type Boolean))
  (bind _cell (Processing|GetCell Coords))
  (if (and (Conversions|AreCoordsValid Coords) (!= Alive (.alive _cell)))
    (if Is%20Canvas%20Ready
      (LocalVariables|SetDeltaN (Math|Integer|SelectInt 1 -1 Alive) :!label _label)
      (Processing|SetCell Coords (Utilities|Struct|MakeS_Cell (.n-count _cell) Alive))
      (for _index (range -1 1)
        (for _index_2 (range -1 1)
          (if (and (Conversions|AreCoordsValid (Utilities|Struct|MakeIntPoint (+ _index_2 (.x Coords)) (+ _index (.y Coords)))) (!= (Utilities|Struct|MakeIntPoint (+ _index_2 (.x Coords)) (+ _index (.y Coords))) Coords))
            (Processing|SetCell (Utilities|Struct|MakeIntPoint (+ _index_2 (.x Coords)) (+ _index (.y Coords))) (Utilities|Struct|MakeS_Cell (+ (LocalVariables|GetDeltaN) (.n-count (Processing|GetCell (Utilities|Struct|MakeIntPoint (+ _index_2 (.x Coords)) (+ _index (.y Coords)))))) (.alive (Processing|GetCell (Utilities|Struct|MakeIntPoint (+ _index_2 (.x Coords)) (+ _index (.y Coords))))))))))
      (else
        (bind (_canvas _size _context) (Rendering|BeginDrawCanvastoRenderTarget (Variables|Buffers|GetBuffer%20Target)))
        (Variables|Materials|SetCanvas _canvas)
        (Utilities|FlowControl|Sequence
          (:then_0
            (goto _label))
          (:then_1
            (Rendering|EndDrawCanvastoRenderTarget _context)))))))

(fn ComputeCellState
  (params (Cell :type S%20Cell%20Structure))
  (return (or (== (.n-count Cell) 3) (and (== (.n-count Cell) 2) (.alive Cell)))))

(fn ComputeCellBuffer
  (bind (_canvas _size _context) (Rendering|BeginDrawCanvastoRenderTarget (Variables|Buffers|GetBuffer%20Target)))
  (Variables|Materials|SetCanvas _canvas)
  (bind _output_get (LocalVariables|SetBuffer%20Copy (Variables|Buffers|GetCellsBuffer)))
  (bind _keys (Utilities|Map|Keys _output_get))
  (for _array_element _keys
    (Processing|SetCellState (Processing|ComputeCellState (Conversions|BytetoCell (.Value (Utilities|Map|Find (LocalVariables|GetBuffer%20Copy) _array_element)))) _array_element true))
  (Rendering|EndDrawCanvastoRenderTarget _context))

(fn InitBufferSize
  (bind _returnvalue (Viewport|GetViewportSize))
  (bind _buffer_size (Variables|Options|GetBuffer%20Size))
  (bind _buffer_size_2 (Variables|Options|GetBuffer%20Size))
  (bind _returnvalue_2 (Class|KismetMathLibrary|ToIntPoint(Vector2D) _returnvalue))
  (Variables|Buffers|SetCanvas%20Size (Utilities|Struct|MakeIntPoint (Math|Integer|SelectInt (.x _returnvalue_2) (.x _buffer_size_2) (<= (.x _buffer_size) 0)) (Math|Integer|SelectInt (.y _returnvalue_2) (.y _buffer_size_2) (<= (.y _buffer_size) 0)))))

(fn SetupRenderTarget
  (bind _canvas_size (Variables|Buffers|GetCanvas%20Size))
  (bind _canvas_size_2 (Variables|Buffers|GetCanvas%20Size))
  (bind _canvas_size_3 (Variables|Buffers|GetCanvas%20Size))
  (bind _returnvalue (Math|Conversions|ToVector2D(IntPoint) _canvas_size_3))
  (bind (_x _y) (Math|Vector2D|BreakVector2D _returnvalue))
  (bind _returnvalue_2 (/ "(X=1.000000,Y=1.000000)" _returnvalue))
  (Utilities|FlowControl|Sequence
    (:then_0
      (bind _returnvalue_3 (CanvasRenderTarget2D|CreateCanvasRenderTarget2D "/Script/Engine.CanvasRenderTarget2D" (.x _canvas_size_2) (.y _canvas_size_2)))
      (Utilities|IsValid _returnvalue_3
        (:Is%20Valid
          (bind _output_get (Variables|Buffers|SetDisplay%20Target _returnvalue_3))
          (Variables|/Script/Engine.Texture|SetLODGroup _output_get "TEXTUREGROUP_Pixels2D")
          (Variables|/Script/Engine.TextureRenderTarget2D|SetAddressX _output_get "TA_Clamp")
          (Variables|/Script/Engine.TextureRenderTarget2D|SetAddressY _output_get "TA_Clamp"))))
    (:then_1
      (bind _returnvalue_4 (CanvasRenderTarget2D|CreateCanvasRenderTarget2D "/Script/Engine.CanvasRenderTarget2D" (.x _canvas_size) (.y _canvas_size)))
      (Utilities|IsValid _returnvalue_4
        (:Is%20Valid
          (bind _output_get_2 (Variables|Buffers|SetBuffer%20Target _returnvalue_4))
          (Variables|/Script/Engine.Texture|SetLODGroup _output_get_2 "TEXTUREGROUP_Pixels2D")
          (Variables|/Script/Engine.TextureRenderTarget2D|SetAddressX _output_get_2 "TA_Clamp")
          (Variables|/Script/Engine.TextureRenderTarget2D|SetAddressY _output_get_2 "TA_Clamp"))))
    (:then_2
      (bind _returnvalue_5 (Rendering|Material|CreateDynamicMaterialInstance "/Game/Conway/M_ComputeConway.M_ComputeConway" "None" "None" :!class /Script/Engine.KismetMaterialLibrary))
      (bind _output_get_3 (Variables|Materials|SetCompute%20Material _returnvalue_5))
      (Rendering|Material|SetTextureParameterValue _output_get_3 "ComputeBuffer" (Variables|Buffers|GetBuffer%20Target))
      (Rendering|Material|SetVectorParameterValue _output_get_3 "BufferSize" (Math|Color|MakeColor _x _y (.x _returnvalue_2) (.y _returnvalue_2)) :!class /Script/Engine.MaterialInstanceDynamic)
      (bind _returnvalue_6 (Rendering|Material|CreateDynamicMaterialInstance "/Game/Conway/M_RenderConway.M_RenderConway" "None" "None" :!class /Script/Engine.KismetMaterialLibrary))
      (bind _output_get_4 (Variables|Materials|SetRender%20Material _returnvalue_6))
      (Rendering|Material|SetTextureParameterValue _output_get_4 "ComputeBuffer" (Variables|Buffers|GetBuffer%20Target)))))

(fn DrawCurrentState
  (bind _display_target (Variables|Buffers|GetDisplay%20Target))
  (Utilities|IsValid _display_target
    (:Is%20Valid
      (bind (_canvas _size _context) (Rendering|BeginDrawCanvastoRenderTarget _display_target))
      (Canvas|DrawMaterial :self _canvas :RenderMaterial (Variables|Materials|GetRender%20Material) :ScreenSize _size :CoordinateSize "(X=1.000000,Y=1.000000)" :PivotPoint "(X=0.500000,Y=0.500000)")
      (Rendering|EndDrawCanvastoRenderTarget _context))))