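; Showcase actor that moves its mesh along a spline from BeginPlay, with looping and direction switching.
; A timeline, rate-scaled by MovementDuration, supplies a linear or smooth alpha that sets the mesh's local spline location and rotation with sweep.
; When the timeline finishes, StartMovement calls itself, choosing forward or reverse playback from the last direction and ReverseAtEnd.
; A loop count limits repeats, with zero or less meaning endless.
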(event Custom|StartMovement
  (params (Forward :type Boolean))
  (bind _number_of_loops (Variables|MovementOptions|GetNumber%20Of%20Loops))
  (bind _pathspline (Variables|Default|GetPathSpline))
  (bind _output_get (Variables|Checks|SetIsReverse Forward))
  (if _output_get
    (bind (_direction _alphasmooth _alphalinear) (Timeline|MovementTimeline PlayFromStart)
      (:Update
        (Transformation|SetRelativeLocationAndRotation (Variables|Default|GetVisibleMesh) (Spline|GetLocationatTime _pathspline (* (select (Variables|MovementOptions|GetLinear%20Movement) _alphalinear _alphasmooth) (Variables|/Script/Engine.SplineComponent|GetDuration (Variables|Default|GetPathSpline))) "Local" false) (Class|SplineComponent|GetRotationatTime _pathspline (* (select (Variables|MovementOptions|GetLinear%20Movement) _alphalinear _alphasmooth) (Variables|/Script/Engine.SplineComponent|GetDuration (Variables|Default|GetPathSpline))) "Local" false) true false))
      (:Finished
        ;[1 1 1] Restart Movement
        (if true
          (bind _result (Math|Integer|IncrementInt (Variables|Checks|GetLoop%20Iterator))
            (:%20%20
              _)))
        (if (or (or (<= _result _number_of_loops) (<= _number_of_loops 0)) (and (== (Variables|MovementOptions|GetNumber%20Of%20Loops) (Variables|MovementOptions|GetNumber%20Of%20Loops)) (not (Variables|Checks|GetIsReverse))))
          (CallFunction|StartMovement (and (not (Variables|Checks|GetIsReverse)) (Variables|MovementOptions|GetReverse%20At%20End))))))
    (else
      (Timeline|MovementTimeline ReverseFromEnd))))

(event EventBeginPlay
  (Components|Timeline|SetPlayRate (Variables|Default|GetMovementTimeline) (/ 512.0 (Math|Float|Max(Float) (Variables|MovementOptions|GetMovement%20Duration) 0.01)))
  (CallFunction|StartMovement true))

(fn ConstructionScript)