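; BP_FourWayCase is a showcase actor that sets up masked-window materials on a cylinder, cube and sphere framed by four pillars.
; On BeginPlay it creates a dynamic M_MaskedWindow instance for each shape with its own base color.
; Each instance receives two adjacent pillars' world positions as left and right window bounds, giving each shape a different side of the case.
; The side between Pillar1 and Pillar2 has no shape assigned.
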(event EventBeginPlay
  (Utilities|FlowControl|Sequence
    (:then_0
      (bind _returnvalue (Rendering|Material|CreateDynamicMaterialInstance "/Game/Materials/Surface/M_MaskedWindow.M_MaskedWindow" "None" "None" :!class /Script/Engine.KismetMaterialLibrary))
      (bind _output_get (Variables|MaterialInstances|SetCylinderMat _returnvalue))
      (Rendering|Material|SetVectorParameterValue _output_get "Window Left" (Math|Conversions|ToLinearColor(Vector) (Transformation|GetWorldLocation (Variables|Default|GetPillar2))) :!class /Script/Engine.MaterialInstanceDynamic)
      (Rendering|Material|SetVectorParameterValue _output_get "Window Right" (Math|Conversions|ToLinearColor(Vector) (Transformation|GetWorldLocation (Variables|Default|GetPillar3))) :!class /Script/Engine.MaterialInstanceDynamic)
      (Rendering|Material|SetVectorParameterValue _output_get "Base Color" (Variables|Default|GetCylinderColor) :!class /Script/Engine.MaterialInstanceDynamic)
      (Rendering|Material|SetMaterial (Variables|Default|GetCylinder) 0 _output_get))
    (:then_1
      (bind _returnvalue_2 (Rendering|Material|CreateDynamicMaterialInstance "/Game/Materials/Surface/M_MaskedWindow.M_MaskedWindow" "None" "None" :!class /Script/Engine.KismetMaterialLibrary))
      (bind _output_get_2 (Variables|MaterialInstances|SetCubeMat _returnvalue_2))
      (Rendering|Material|SetVectorParameterValue _output_get_2 "Window Left" (Math|Conversions|ToLinearColor(Vector) (Transformation|GetWorldLocation (Variables|Default|GetPillar3))) :!class /Script/Engine.MaterialInstanceDynamic)
      (Rendering|Material|SetVectorParameterValue _output_get_2 "Window Right" (Math|Conversions|ToLinearColor(Vector) (Transformation|GetWorldLocation (Variables|Default|GetPillar4))) :!class /Script/Engine.MaterialInstanceDynamic)
      (Rendering|Material|SetVectorParameterValue _output_get_2 "Base Color" (Variables|Default|GetCubeColor) :!class /Script/Engine.MaterialInstanceDynamic)
      (Rendering|Material|SetMaterial (Variables|Default|GetCube) 0 _output_get_2))
    (:then_2
      (bind _returnvalue_3 (Rendering|Material|CreateDynamicMaterialInstance "/Game/Materials/Surface/M_MaskedWindow.M_MaskedWindow" "None" "None" :!class /Script/Engine.KismetMaterialLibrary))
      (bind _output_get_3 (Variables|MaterialInstances|SetSphereMat _returnvalue_3))
      (Rendering|Material|SetVectorParameterValue _output_get_3 "Window Left" (Math|Conversions|ToLinearColor(Vector) (Transformation|GetWorldLocation (Variables|Default|GetPillar4))) :!class /Script/Engine.MaterialInstanceDynamic)
      (Rendering|Material|SetVectorParameterValue _output_get_3 "Window Right" (Math|Conversions|ToLinearColor(Vector) (Transformation|GetWorldLocation (Variables|Default|GetPillar1))) :!class /Script/Engine.MaterialInstanceDynamic)
      (Rendering|Material|SetVectorParameterValue _output_get_3 "Base Color" (Variables|Default|GetSphereColor) :!class /Script/Engine.MaterialInstanceDynamic)
      (Rendering|Material|SetMaterial (Variables|Default|GetSphere) 0 _output_get_3))))

(fn ConstructionScript)